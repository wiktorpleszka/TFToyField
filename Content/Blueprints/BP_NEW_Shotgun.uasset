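; Shotgun weapon Blueprint that fires hitscan shots from the player camera when the Shoot axis event runs.
; Each shot repeats an identical, spread-free camera-forward line trace ten times, applying damage and spawning a muzzle flash emitter at each hit location.
; A fire sound plays at the weapon, and a DoOnce reset after the RateOfFire delay throttles the per-frame axis event, whose value is never checked.
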(event `InputAxis|Shoot`
  (params (AxisValue :type "Float (single-precision)"))
  (bind _transformcomponent (`PlayerCameraManager.TransformComponent` (`GameplayStatics.GetPlayerCameraManager` 0)))
  (bind _returnvalue (`SceneComponent.K2_GetComponentLocation` _transformcomponent))
  (`/Engine/EditorBlueprintResources/StandardMacros.DoOnce` false :!label _label
    (:`Completed`
      (`|ExecutionSequence`
        (:`then_0`
          (for _ (range 1 11)
            (bind _outhit (`KismetSystemLibrary.LineTraceSingle` _returnvalue (+ _returnvalue (* (`SceneComponent.GetForwardVector` _transformcomponent) (`self.Distance`))) "TraceTypeQuery2" false (`|MakeArray` (`self.Character`) :!type "Actor Object Reference") "ForDuration"))
            (if true
              (bind (_bblockinghit _binitialoverlap _time _distance _location _impactpoint _normal _impactnormal _physmat _hitactor) (`GameplayStatics.BreakHitResult` _outhit))
              (`GameplayStatics.SpawnEmitterAtLocation` "/Game/MilitaryWeapSilver/FX/P_Shotgun_MuzzleFlash_01.P_Shotgun_MuzzleFlash_01" _location)
              (`GameplayStatics.ApplyDamage` _hitactor (`self.Damage`))
              (`GameplayStatics.PlaySoundAtLocation` null _location (struct) 1.0 1.0 0.0 null null null null)))
          (`GameplayStatics.PlaySoundAtLocation` "/Game/MilitaryWeapSilver/Sound/Shotgun/Wavs/ShotgunA_Fire01.ShotgunA_Fire01" (`self.K2_GetActorLocation`) (struct) 1.0 1.0 0.0 null null null null))
        (:`then_1`
          (`KismetSystemLibrary.Delay` (`self.RateOfFire`))
          (goto _label :!via `Reset`))))))

(fn `UserConstructionScript`)